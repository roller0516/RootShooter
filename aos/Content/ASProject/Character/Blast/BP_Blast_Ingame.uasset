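; Blast's in-game character Blueprint, adding footprint spawning and grappling-hook input.
; SpawnFootPrintL and SpawnFootPrintR events spawn left and right footprint actors at the FootL and FootR components, scaled down and aligned to the actor's rotation.
; The Enhanced Input IA_Grapping action calls AttemptGrapple on the GrappleHookComponent whenever it triggers.
; BeginPlay, Tick, overlap and the construction script are empty, and nothing in this graph calls the footprint events.
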(event `self.ReceiveBeginPlay`)

(event `Spawn FootPrint L`
  (`|SpawnActorFromClass` "/Game/ASProject/FootPrint/BP_LFootPrint.BP_LFootPrint_C" (`KismetMathLibrary.MakeTransform` (`SceneComponent.K2_GetComponentLocation` (`self.Foot_L`)) (`self.K2_GetActorRotation`) (0.1 0.1 0.1)) "Undefined" "OverrideRootScale" null null))

(event `Spawn FootPrint R`
  (`|SpawnActorFromClass` "/Game/ASProject/FootPrint/BP_RFootPrint.BP_RFootPrint_C" (`KismetMathLibrary.MakeTransform` (`SceneComponent.K2_GetComponentLocation` (`self.Foot_R`)) (`self.K2_GetActorRotation`) (0.1 0.1 0.1)) "Undefined" "OverrideRootScale" null null))

(event `EnhancedInput|/Game/ASProject/Character/Input/Actions/IA_Grapping`
  (params (ActionValue :type Boolean) (ElapsedSeconds :type "Float (double-precision)") (TriggeredSeconds :type "Float (double-precision)") (InputAction :type "InputAction Object Reference" :default "/Game/ASProject/Character/Input/Actions/IA_Grapping.IA_Grapping"))
  (:`Triggered`
    (`/Game/ASProject/GrappleHookSystem/GrappleHook_Component.AttemptGrapple` (`self.GrappleHook_Component`))))

(fn `UserConstructionScript`)