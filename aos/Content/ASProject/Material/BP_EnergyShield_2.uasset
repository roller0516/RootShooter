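; BP_EnergyShield_2 is an energy shield actor that plays a timed appear, blink and dissolve sequence on its sphere mesh, entirely through material parameters.
; After a short delay on BeginPlay it creates a dynamic material instance, and a show timeline animates DissolveAmount.
; After a pause it sets a Destroy flag, then chains a blink timeline driving TimeSpeed into a destroy timeline driving DissolveAmount.
; The actor itself is never destroyed.
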(event `self.ReceiveBeginPlay`
  (bind _sphere (`self.Sphere`))
  (`KismetSystemLibrary.Delay` 2.0)
  (bind _returnvalue (`PrimitiveComponent.CreateDynamicMaterialInstance` _sphere 0 (`PrimitiveComponent.GetMaterial` _sphere 0) "None"))
  (bind (_direction `_새_트랙_0`) (`Timeline|TL_Show`)
    (:`Update`
      (`MaterialInstanceDynamic.SetScalarParameterValue` _returnvalue "DissolveAmount" `_새_트랙_0`))
    (:`Finished`
      (`KismetSystemLibrary.Delay` 5.0)
      (`MaterialInstanceDynamic.SetScalarParameterValue` _returnvalue "Destroy" 1.0)
      (bind (_direction_2 `_새_트랙_0_2`) (`Timeline|TL_Blink` :!via `PlayFromStart`)
        (:`Update`
          (`MaterialInstanceDynamic.SetScalarParameterValue` _returnvalue "TimeSpeed" `_새_트랙_0_2`))
        (:`Finished`
          (bind (_direction_3 `_새_트랙_0_3`) (`Timeline|TL_Destroy` :!via `PlayFromStart`)
            (:`Update`
              (`MaterialInstanceDynamic.SetScalarParameterValue` _returnvalue "DissolveAmount" `_새_트랙_0_3`))))))))

(fn `UserConstructionScript`)