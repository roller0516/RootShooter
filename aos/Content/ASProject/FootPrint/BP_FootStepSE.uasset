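; Footstep anim notify that plays a surface-dependent sound and raises a noise event for AI hearing.
; A downward line trace from the owning actor finds the surface type, which selects between default, rock and water sounds attached to the mesh.
; Owner speed scales volume and pitch, both multiplied by StepSound, which also sets the loudness of the "Detected"-tagged noise at the hit point.
; Debug prints report whether the trace hit.
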(fn `Received_Notify`
  (params (MeshComp :type "SkeletalMeshComponent Object Reference") (Animation :type "AnimSequenceBase Object Reference") (EventReference :type "AnimNotifyEventReference Structure (by ref)"))
  (returns (ReturnValue :type Boolean))
  (bind _returnvalue (`ActorComponent.GetOwner` MeshComp))
  (bind _returnvalue_2 (`Actor.K2_GetActorLocation` _returnvalue))
  (bind (_x _y _z) (`KismetMathLibrary.BreakVector3f` _returnvalue_2))
  (bind _returnvalue_3 (* (`KismetMathLibrary.MapRangeClamped` (`KismetMathLibrary.VSize` (`Actor.GetVelocity` _returnvalue)) 0.0 500.0 0.0 1.0) (`self.StepSound`)))
  (bind (_outhit _returnvalue_4) (`KismetSystemLibrary.LineTraceSingle` _returnvalue_2 (`KismetMathLibrary.MakeVector` _x _y (- _z 500.0)) "TraceTypeQuery1" false (`|MakeArray` _returnvalue)))
  (if _returnvalue_4
    (`GameplayStatics.SpawnSoundAttached` (select `EPhysicalSurface` (`GameplayStatics.GetSurfaceType` _outhit) :!type "SoundBase Object Reference") (`local.MeshComp`) "None" (0.0 0.0 0.0) (struct) "KeepRelativeOffset" false _returnvalue_3 _returnvalue_3 0.0 null null)
    (`AISense_Hearing.ReportNoiseEvent` (`.Location` (`GameplayStatics.BreakHitResult` _outhit)) (`self.StepSound`) null 0.0 "Detected")
    (`KismetSystemLibrary.PrintString` "Foot")
    (return false)
    (else
      (`KismetSystemLibrary.PrintString` "Foot False")
      (return false))))