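; Grappling hook component for the third-person character that picks and highlights the best grapple target in range.
; Tick switches on grapple state; only the inactive state has logic, while Firing, Near Target and Hit Target are empty stubs.
; It sphere-overlaps for hook targets, keeps those with clear line of sight and chooses the smallest angle from character forward.
; Changing target deactivates the old one and activates the new; traces leave persistent debug lines.
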(event `self.ReceiveBeginPlay`
  (cast `/Game/ThirdPerson/Blueprints/BP_ThirdPersonCharacter` (`self.GetOwner`)))

(event `self.ReceiveTick`
  (params (DeltaSeconds :type "Float (single-precision)"))
  (switch `/Game/ASProject/GrappingHookSystem/E_GrappleState` (`self.GrappleState`)
    (:`NewEnumerator0`
      (`self.InActive`))
    (:`NewEnumerator1`
      (`self.Firing`))
    (:`NewEnumerator2`
      (`self.NearTarget`))
    (:`NewEnumerator3`
      (`self.HitTarget`))))

(fn `FindBestTarget`
  (params (Targets :type "Array of Actor Object Reference"))
  (returns (Target :type "Actor Object Reference"))
  (locals (`CurrentTarget(Local)` :type "Actor Object Reference") (`CurrentAngle(Local)` :type "Float (double-precision)" :default 0.0) (`BestAngle(Local)` :type "Float (double-precision)") (`BestTarget(Local)` :type "Actor Object Reference"))
  (bind _owningcharacter (`self.OwningCharacter`))
  (for _array_element Targets
    (set `local.CurrentTarget(Local)` _array_element)
    (bind _outhit (`KismetSystemLibrary.LineTraceSingle` (`Actor.K2_GetActorLocation` (`self.OwningCharacter`)) (`Actor.K2_GetActorLocation` (`local.CurrentTarget(Local)`)) "TraceTypeQuery1" false (`|MakeArray` (`self.OwningCharacter`) :!type "aosCharacter Object Reference") "Persistent" true (struct :`R` 1.0 :`A` 1.0) (struct :`G` 1.0 :`A` 1.0) 0.5))
    (if (== (`.HitActor` (`GameplayStatics.BreakHitResult` _outhit)) (`local.CurrentTarget(Local)`))
      (`|ExecutionSequence`
        (:`then_0`
          ;[1 1 1] step1 calculate angle to target
          (set `local.CurrentAngle(Local)` (`KismetMathLibrary.DegAcos` (`KismetMathLibrary.Dot_VectorVector` (`KismetMathLibrary.Normal` (- (`Actor.K2_GetActorLocation` (`local.CurrentTarget(Local)`)) (`Actor.K2_GetActorLocation` _owningcharacter))) (`SceneComponent.GetForwardVector` (`Actor.RootComponent` _owningcharacter))))))
        (:`then_1`
          ;[1 1 1] step2 if the angle is less than the current angle or there is not best target, make this the next target
          (if (or (< (`local.CurrentAngle(Local)`) (`local.BestAngle(Local)`)) (not (`KismetSystemLibrary.IsValid` (`local.BestTarget(Local)`))))
            (set `local.BestTarget(Local)` (`local.CurrentTarget(Local)`))
            (set `local.BestAngle(Local)` (`local.CurrentAngle(Local)`)))))))
  (return (`local.BestTarget(Local)`)))

(fn `Firing`)

(fn `HitTarget`)

(fn `InActive`
  (bind _outactors (`KismetSystemLibrary.SphereOverlapActors` (`Actor.K2_GetActorLocation` (`self.OwningCharacter`)) (`self.MaxGrappleDistance`) (`|MakeArray` "ObjectTypeQuery1" :!type "EObjectTypeQuery Enum") "/Game/ASProject/GrappingHookSystem/BP_GrappleHookTarget.BP_GrappleHookTarget_C"))
  (bind _target (`self.FindBestTarget` _outactors))
  (`self.SetCurrentTarget` (cast `/Game/ASProject/GrappingHookSystem/BP_GrappleHookTarget` _target :!pure true)))

(fn `NearTarget`)

(fn `SetCurrentTarget`
  (params (NewTarget :type "/Game/ASProject/GrappingHookSystem/BP_GrappleHookTarget Object Reference"))
  (if (!= NewTarget (`self.CurrentTarget`))
    (`|ExecutionSequence`
      (:`then_0`
        ;[1 1 1] Hide Old Target
        (bind _currenttarget (`self.CurrentTarget`)
          (:`then`
            (`/Game/ASProject/GrappingHookSystem/BP_GrappleHookTarget.SetActive` _currenttarget false))
          (:`else`)))
      (:`then_1`
        ;[1 1 1] Set New Target
        (set `self.CurrentTarget` (`local.NewTarget`)))
      (:`then_2`
        ;[1 1 1] Show New Target
        (bind _currenttarget_2 (`self.CurrentTarget`)
          (:`then`
            (`/Game/ASProject/GrappingHookSystem/BP_GrappleHookTarget.SetActive` _currenttarget_2 true))
          (:`else`))))))