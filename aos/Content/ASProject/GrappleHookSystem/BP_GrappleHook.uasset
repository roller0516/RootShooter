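; BP_GrappleHook is the grapple hook actor that flies in a straight line to its Target and stops there.
; BeginPlay caches start and end points and sets the ProjectileMovement velocity along that direction at HookSpeed.
; Tick compares squared distances from the start against the Target's current location, then snaps the hook to the cached end point and zeroes velocity.
; DistanceToTarget reports the remaining distance to that cached end point.
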(event `self.ReceiveBeginPlay`
  (set `self.StartingLocation` (`self.K2_GetActorLocation`))
  (set `self.EndingLocation` (`self.K2_GetActorLocation` (`self.Target`)))
  (set `self.Direction` (`KismetMathLibrary.Normal` (- (`self.EndingLocation`) (`self.StartingLocation`))))
  (set `MovementComponent.Velocity` (* (`self.Direction`) (`self.HookSpeed`)) (`self.ProjectileMovement`)))

(event `self.ReceiveTick`
  (params (DeltaSeconds :type "Float (single-precision)"))
  (if (>= (`KismetMathLibrary.Vector_DistanceSquared` (`self.K2_GetActorLocation`) (`self.StartingLocation`)) (`KismetMathLibrary.Vector_DistanceSquared` (`self.K2_GetActorLocation` (`self.Target`)) (`self.StartingLocation`)))
    (`self.K2_SetActorLocation` (+ (`self.StartingLocation`) (* (`self.Direction`) (`KismetMathLibrary.Vector_Distance` (`self.StartingLocation`) (`self.EndingLocation`)))))
    (set `MovementComponent.Velocity` (0.0 0.0 0.0) (`self.ProjectileMovement`))))

(fn `DistanceToTarget`
  (returns (ReturnValue :type "Float (double-precision)"))
  (return (`KismetMathLibrary.Vector_Distance` (`self.EndingLocation`) (`self.K2_GetActorLocation`))))

(fn `UserConstructionScript`)