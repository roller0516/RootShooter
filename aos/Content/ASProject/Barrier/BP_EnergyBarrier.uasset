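; Energy barrier actor that dissolves in on spawn, warns before expiring, and removes itself.
; Timelines drive a dynamic sphere material: show dissolve, a ten-second delay, blinking via TimeSpeed, then a destroy dissolve.
; DestroyActor fires from the final timeline's Update rather than Finished, cutting that dissolve short.
; Each hit on Sphere2 adds a child actor at the sphere's scale and passes it the impact point.
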(event `self.ReceiveBeginPlay`
  (bind _sphere (`self.Sphere`))
  (bind _returnvalue (`PrimitiveComponent.CreateDynamicMaterialInstance` _sphere 0 (`PrimitiveComponent.GetMaterial` _sphere 0) "None"))
  (bind (_direction `_새_트랙_0`) (`Timeline|TL_Show`)
    (:`Update`
      (`MaterialInstanceDynamic.SetScalarParameterValue` _returnvalue "DissolveAmount" `_새_트랙_0`)
      (`KismetSystemLibrary.Delay` 10.0)
      (`MaterialInstanceDynamic.SetScalarParameterValue` _returnvalue "Destroy" 1.0)
      (bind (_direction_2 `_새_트랙_0_2`) (`Timeline|TL_Blink` :!via `PlayFromStart`)
        (:`Update`
          (`MaterialInstanceDynamic.SetScalarParameterValue` _returnvalue "TimeSpeed" `_새_트랙_0_2`))
        (:`Finished`
          (bind (_direction_3 `_새_트랙_0_3`) (`Timeline|TL_Destroy` :!via `PlayFromStart`)
            (:`Update`
              (`MaterialInstanceDynamic.SetScalarParameterValue` _returnvalue "DissolveAmount" `_새_트랙_0_3`)
              (`self.K2_DestroyActor`))))))))

(event `self.Sphere2.OnComponentHit`
  (params (HitComponent :type "PrimitiveComponent Object Reference") (OtherActor :type "Actor Object Reference") (OtherComp :type "PrimitiveComponent Object Reference") (NormalImpulse :type "Vector Structure") (Hit :type "HitResult Structure (by ref)"))
  (bind _returnvalue (`AddComponent|NODE_AddChildActorComponent-1` :`RelativeTransform` (`KismetMathLibrary.MakeTransform` (0.0 0.0 0.0) (struct) (`SceneComponent.K2_GetComponentScale` (`self.Sphere`)))))
  (message `/Game/ASProject/Barrier/BPI_ImpactPoint.Impact_point` (`ChildActorComponent.ChildActor` _returnvalue) Hit_ImpactPoint))

(fn `UserConstructionScript`)